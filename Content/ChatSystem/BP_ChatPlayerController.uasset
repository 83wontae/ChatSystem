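; BP_ChatPlayerController is the player controller for the chat system, linking chat input and messages to BP_ChatHUD.
; Pressing Enter focuses the chat through the HUD.
; ReqChatMessage passes a sender name and message directly to ResChatMessage, which adds them to the chat via the HUD.
; Both HUD calls cast the HUD of player controller 0 rather than the controller's own.
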(event `Key|Enter`
  (params (Key :type "Key Structure"))
  (:`Pressed`
    (bind _asbp_chat_hud (cast `/Game/ChatSystem/BP_ChatHUD` (`self.GetHUD` (`GameplayStatics.GetPlayerController` 0))))
    (`/Game/ChatSystem/BP_ChatHUD.FocusChat` _asbp_chat_hud)))

(event `ReqChatMessage`
  (params (Name :type Text) (Message :type Text))
  (`self.ResChatMessage` Name Message))

(event `ResChatMessage`
  (params (Name :type Text) (Message :type Text))
  (bind _asbp_chat_hud (cast `/Game/ChatSystem/BP_ChatHUD` (`self.GetHUD` (`GameplayStatics.GetPlayerController` 0))))
  (`/Game/ChatSystem/BP_ChatHUD.AddChat` _asbp_chat_hud Name Message))

(fn `UserConstructionScript`)